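; BP_Sakti is a player-controlled pawn Blueprint that handles basic movement and mouse look through input axis events.
; Forward/backward input moves it along the control rotation's yaw, and right/left input along the right vector from control yaw and roll.
; Mouse axes feed controller pitch and yaw directly, so looking steers the movement direction.
; The construction script is empty.
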(event Input|AxisEvents|InputAxisForwards/Backwards
  (params (AxisValue :type Float%20%28single-precision%29))
  ;[0 0 0] Movement
  (Pawn|Input|AddMovementInput (Math|Vector|GetForwardVector (Math|Rotator|MakeRotator 0.0 0.0 (.yaw (Pawn|GetControlRotation :!class /Script/Engine.Pawn)))) AxisValue false))

(event Input|AxisEvents|InputAxisRight/Left
  (params (AxisValue :type Float%20%28single-precision%29))
  (bind _returnvalue (Pawn|GetControlRotation :!class /Script/Engine.Pawn))
  ;[0 0 0] Movement
  (Pawn|Input|AddMovementInput (Math|Vector|GetRightVector (Math|Rotator|MakeRotator (.roll _returnvalue) 0.0 (.yaw _returnvalue))) AxisValue false))

(event Input|AxisEvents|InputAxisMouseUp/Down
  (params (AxisValue :type Float%20%28single-precision%29))
  ;[0 0 0] Mouse
  (Pawn|Input|AddControllerPitchInput AxisValue))

(event Input|AxisEvents|InputAxisMouseRight/Left
  (params (AxisValue :type Float%20%28single-precision%29))
  ;[0 0 0] Mouse
  (Pawn|Input|AddControllerYawInput AxisValue))

(fn ConstructionScript)