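; NPC quest giver that holds data-table-driven conversations with the player character BP_Sakti.
; BeginPlay caches dialogue rows matching its NPCID, and a box overlap toggles an interact text prompt.
; Each Interact advances the line in a WB_Dialog widget, turns the NPC toward the player and calls AcceptQuest, swapping the exclamation marker for a question mark.
; The camera blends to the NPC during dialogue and back when lines run out, overlap ends or chat closes.
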(event OnComponentBeginOverlap(Box)
  (params (OverlappedComponent :type Primitive%20Component%20Object%20Reference) (OtherActor :type Actor%20Object%20Reference) (OtherComp :type Primitive%20Component%20Object%20Reference) (OtherBodyIndex :type Integer) (bFromSweep :type Boolean) (SweepResult :type Hit%20Result%20Structure%20%28by%20ref%29))
  ;[1 1 1] Show Interact
  (Utilities|Casting|CastToBP_Sakti OtherActor)
  (Development|SetHiddeninGame (Variables|Default|GetTextRender) false false))

(event OnComponentEndOverlap(Box)
  (params (OverlappedComponent :type Primitive%20Component%20Object%20Reference) (OtherActor :type Actor%20Object%20Reference) (OtherComp :type Primitive%20Component%20Object%20Reference) (OtherBodyIndex :type Integer))
  ;[1 1 1] Show Interact
  (Utilities|Casting|CastToBP_Sakti OtherActor)
  (Development|SetHiddeninGame (Variables|Default|GetTextRender) true false))

(event Custom|PlayerAdjusmnent
  (bind _returnvalue (Game|GetPlayerController 0))
  (Variables|/Script/Engine.PlayerController|SetbShowMouseCursor _returnvalue true)
  (Input|SetInputModeUIOnly _returnvalue 0 "DoNotLock" false)
  (Pawn|Components|CharacterMovement|DisableMovement (Variables|/Script/Engine.Character|GetCharacterMovement (Game|GetPlayerCharacter 0))))

(event Custom|EventQuestComplete
  ;[1 1 1] Quest Complete
  (Variables|/Game/JINAWI/Blueprints/QuestSystem/NPC_Dialogue.NPC_Dialogue_C|SetQuestFinished (Variables|Default|GetNPCChat) true)
  (Rendering|Material|SetMaterial (Variables|Default|GetQuestionmrk) 0 0)
  (Variables|Default|SetQuestComplete true))

(event Custom|EndChat
  ;[1 1 1] End Chat
  (bind _returnvalue (UserInterface|CreateWidget "/Game/JINAWI/Blueprints/NPC/Dialogue/BlackScreenPop.BlackScreenPop_C"))
  (UserInterface|Viewport|AddtoViewport _returnvalue 0)
  (Utilities|FlowControl|Delay 0.2)
  (Widget|RemovefromParent (Variables|Default|GetNPCChat))
  (Game|Player|SetViewTargetwithBlend (Game|GetPlayerController 0) (.AsBP%20Sakti (Utilities|Casting|CastToBP_Sakti (Game|GetPlayerCharacter 0))) 2.0 "VTBlend_Linear" 0.0 false)
  (Widget|RemovefromParent (Variables|Default|GetDialogueWidget))
  (Variables|Default|SetDialogueWidget 0))

(event Custom|AcceptQuest
  ;[1 1 1] Accept Quest
  (Development|SetHiddeninGame (Variables|Default|GetQuestionmrk) false false)
  (Development|SetHiddeninGame (Variables|Default|GetExclamationmrk) true false)
  (bind _asbp_sakti (Utilities|Casting|CastToBP_Sakti (Game|GetPlayerCharacter 0)))
  (Default|AcceptQuest _asbp_sakti (Variables|Default|GetQuestRef))
  (Variables|Default|SetQuestActive? true))

(event EventInteract
  (params (QuestLogInfo :type BP%20Quest%20Object%20Reference))
  ;[1 1 1] Intteract
  (Math|Integer|IncrementInt (Variables|Default|GetLineCurrent)
    (:%20%20
      (CallFunction|DialogueCreate)
      (Transformation|SetActorRotation (Math|Rotator|MakeRotator 0.0 0.0 (.Yaw (Math|Rotator|BreakRotator (Math|Rotator|FindLookatRotation (Transformation|GetActorLocation) (Transformation|GetActorLocation (Game|GetPlayerCharacter 0)))))))
      (CallFunction|AcceptQuest))))

(event Collision|EventActorEndOverlap
  (params (OtherActor :type Actor%20Object%20Reference))
  ;[1 1 1] Player Out of trigger
  (bind _asbp_sakti (Utilities|Casting|CastToBP_Sakti OtherActor))
  (Game|Player|SetViewTargetwithBlend (Game|GetPlayerController 0) _asbp_sakti 2.0 "VTBlend_Linear" 0.0 false)
  (Widget|RemovefromParent (Variables|Default|GetDialogueWidget))
  (Variables|Default|SetDialogueWidget 0))

(event EventBeginPlay
  ;[1 1 1] Start Dialog
  (bind _outrownames (DataTable|GetDataTableRowNames "/Game/JINAWI/Blueprints/NPC/Dialogue.Dialogue"))
  (for _array_element _outrownames
    (bind _returnvalue (Utilities|GetDataTableRow "/Game/JINAWI/Blueprints/NPC/Dialogue.Dialogue" _array_element)
      (:then
        (if (== (.NPC_ID (Utilities|Struct|BreakBP_CharacterDialog _returnvalue)) (Variables|Default|GetNPC_ID))
          (Utilities|Array|Add (Variables|Default|GetMyDialogue) _array_element))))))

(fn ConstructionScript)

(fn DialogueCreate
  (bind _returnvalue (Game|GetPlayerController 0))
  (Utilities|IsValid (Variables|Default|GetDialogueWidget)
    (:Is%20Valid
      (bind _returnedline (CallFunction|DialogueGetLine))
      (Variables|/Game/JINAWI/Blueprints/NPC/WB_Dialog.WB_Dialog_C|SetDialogText (Variables|Default|GetDialogueWidget) _returnedline))
    (:Is%20Not%20Valid
      (bind _returnvalue_2 (UserInterface|CreateWidget "/Game/JINAWI/Blueprints/NPC/WB_Dialog.WB_Dialog_C" (Game|GetPlayerController 0)))
      (bind _output_get (Variables|Default|SetDialogueWidget _returnvalue_2))
      (bind _returnedline_2 (CallFunction|DialogueGetLine))
      (Variables|/Game/JINAWI/Blueprints/NPC/WB_Dialog.WB_Dialog_C|SetDialogText _output_get _returnedline_2)
      (Variables|/Game/JINAWI/Blueprints/NPC/WB_Dialog.WB_Dialog_C|SetNameText _output_get (Variables|Default|GetNPC%20Name))
      (UserInterface|Viewport|AddtoViewport _output_get 0)
      (Game|Player|SetViewTargetwithBlend (Game|GetPlayerController 0) self 2.0 "VTBlend_Linear" 0.0 true)
      (Input|SetIgnoreMoveInput _returnvalue false)
      (Input|SetIgnoreLookInput _returnvalue false)
      (Transformation|SetActorRotation (Game|GetPlayerCharacter 0) (Math|Rotator|FindLookatRotation (Transformation|GetActorLocation (Game|GetPlayerCharacter 0)) (Transformation|GetActorLocation)))
      (Transformation|SetActorRotation (Math|Rotator|FindLookatRotation (Transformation|GetActorLocation) (Transformation|GetActorLocation (Game|GetPlayerCharacter 0)))))))

(fn DialogueGetLine
  (bind _returnvalue (Game|GetPlayerController 0))
  (for _array_element (Variables|Default|GetMyDialogue)
    (bind _returnvalue_2 (Utilities|GetDataTableRow "/Game/JINAWI/Blueprints/NPC/Dialogue.Dialogue" _array_element)
      (:then
        (if (and (== (.Conversation_ID (Utilities|Struct|BreakBP_CharacterDialog _returnvalue_2)) (Variables|Default|GetConversation_ID)) (== (.Line_ID (Utilities|Struct|BreakBP_CharacterDialog _returnvalue_2)) (Variables|Default|GetLineCurrent)))
          (Utilities|Array|Add (LocalVariables|GetReturnedLines) (.Dialogue (Utilities|Struct|BreakBP_CharacterDialog _returnvalue_2)))))))
  (if (== (Utilities|Array|Length (LocalVariables|GetReturnedLines)) 1)
    (return (Utilities|Array|Get(acopy) (LocalVariables|GetReturnedLines)))
    (else
      (Widget|RemovefromParent (Variables|Default|GetDialogueWidget))
      (Variables|Default|SetLineCurrent 0)
      (Variables|Default|SetDialogueWidget 0)
      (Game|Player|SetViewTargetwithBlend (Game|GetPlayerController 0) (Game|GetPlayerCharacter 0) 0.0 "VTBlend_Linear" 0.0 false)
      (Input|ResetIgnoreLookInput _returnvalue)
      (Input|ResetIgnoreMoveInput _returnvalue))))

(fn PlayerAdjustments)

(fn BeginChat)