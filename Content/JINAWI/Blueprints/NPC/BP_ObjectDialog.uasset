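; BP_ObjectDialog is an interactable object that shows its own dialog text on screen.
; Interact toggles a WB_Dialog widget: it removes an existing one, or creates one for the first player controller, adds it to the viewport and fills it from MyText.
; When BP_Sakti stops overlapping the actor, the widget is removed and its reference cleared, without a validity check.
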(event Collision|EventActorEndOverlap
  (params (OtherActor :type Actor%20Object%20Reference))
  (Utilities|Casting|CastToBP_Sakti OtherActor)
  (Widget|RemovefromParent (Variables|Default|GetDialogWidget))
  (Variables|Default|SetDialogWidget 0))

(event EventInteract
  (params (QuestLogInfo :type BP%20Quest%20Object%20Reference))
  (Utilities|IsValid (Variables|Default|GetDialogWidget)
    (:Is%20Valid
      (Widget|RemovefromParent (Variables|Default|GetDialogWidget))
      (Variables|Default|SetDialogWidget 0))
    (:Is%20Not%20Valid
      (bind _returnvalue (UserInterface|CreateWidget "/Game/JINAWI/Blueprints/NPC/WB_Dialog.WB_Dialog_C" (Game|GetPlayerController 0)))
      (bind _output_get (Variables|Default|SetDialogWidget _returnvalue))
      (UserInterface|Viewport|AddtoViewport _output_get 0)
      (Variables|/Game/JINAWI/Blueprints/NPC/WB_Dialog.WB_Dialog_C|SetDialogText (Variables|Default|GetDialogWidget) (Variables|Default|GetMy%20Text)))))

(fn ConstructionScript)