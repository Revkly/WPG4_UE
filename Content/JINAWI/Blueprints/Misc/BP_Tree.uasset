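; BP_Tree is a destructible tree actor that stays gone once the game mode records it as destroyed.
; Each Hit Damage call removes one Health regardless of the Damage passed in and reports a successful hit, plus whether the tree died.
; At zero Health it sets IsTreeDestroyed on BP_GameModeMain and destroys itself.
; On BeginPlay it reads that single shared flag and destroys itself if set.
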(event EventBeginPlay
  (bind _asbp_game_mode_main (Utilities|Casting|CastToBP_GameModeMain (Game|GetGameMode)))
  (if (Variables|/Game/JINAWI/Blueprints/Misc/BP_GameModeMain.BP_GameModeMain_C|GetIs%20Tree%20Destroyed _asbp_game_mode_main)
    (Actor|DestroyActor)))

(fn ConstructionScript)

(fn HitDamage
  (params (Damage :type Integer))
  (bind _output_get (Variables|Default|Sethealth (- (Variables|Default|Gethealth) 1)))
  (if (<= _output_get 0)
    (bind _asbp_game_mode_main (Utilities|Casting|CastToBP_GameModeMain (Game|GetGameMode)))
    (Variables|/Game/JINAWI/Blueprints/Misc/BP_GameModeMain.BP_GameModeMain_C|SetIs%20Tree%20Destroyed _asbp_game_mode_main true)
    (Actor|DestroyActor)
    (return true true)
    (else
      (return true false))))