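; Location_BP is a quest location trigger that completes the player's matching quest when reached.
; When BP_Sakti overlaps its box, it searches that character's active quests for any whose actor reference is this location and calls QuestComplete on it.
; It then scans all NPC actors in the level and fires EventQuestComplete on those whose quest name matches the completed one.
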(event OnComponentBeginOverlap(Box)
  (params (OverlappedComponent :type Primitive%20Component%20Object%20Reference) (OtherActor :type Actor%20Object%20Reference) (OtherComp :type Primitive%20Component%20Object%20Reference) (OtherBodyIndex :type Integer) (bFromSweep :type Boolean) (SweepResult :type Hit%20Result%20Structure%20%28by%20ref%29))
  (bind _asbp_sakti (Utilities|Casting|CastToBP_Sakti OtherActor))
  (for _array_element (Variables|/Game/JINAWI/Character/Sakti/BP_Sakti.BP_Sakti_C|GetActiveQuests _asbp_sakti)
    (if (== self (.actorreference (Variables|/Game/JINAWI/Blueprints/QuestSystem/BP_Quest.BP_Quest_C|GetQuestInfo _array_element)))
      (Default|QuestComplete _asbp_sakti 0 _array_element)
      (bind _outactors (Actor|GetAllActorsOfClass "/Game/JINAWI/Blueprints/QuestSystem/NPC.NPC_C"))
      (for _array_element_2 _outactors
        (if (Utilities|Enum|Equal(Enum) (.questname (Variables|/Game/JINAWI/Blueprints/QuestSystem/BP_Quest.BP_Quest_C|GetQuestInfo _array_element)) (.questname (Variables|/Game/JINAWI/Blueprints/QuestSystem/NPC.NPC_C|GetQuestRef _array_element_2)))
          (Default|EventQuestComplete _array_element_2))))))

(fn ConstructionScript)