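; BP_Artifact is a collectible artifact actor that is launched by a physics impulse when it enters play and removed when collected.
; BeginPlay applies a fixed impulse to its Box component.
; Tick spins the static mesh around yaw at a constant, frame-rate-independent speed in world space.
; The Collect event only destroys the actor, with no reward or detection logic in its graphs.
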(event Custom|Collect
  (Actor|DestroyActor))

(event EventBeginPlay
  (Physics|AddImpulse (Variables|Default|GetBox) "25000.000000,50000.000000,25000.000000" "None" false))

(event EventTick
  (params (DeltaSeconds :type Float%20%28single-precision%29))
  (bind _staticmesh (Variables|Default|GetStaticMesh))
  (bind _returnvalue (Transformation|GetWorldRotation _staticmesh))
  (Transformation|SetWorldRotation (Variables|Default|GetStaticMesh) (Math|Rotator|MakeRotator (.roll _returnvalue) (.pitch _returnvalue) (+ (* DeltaSeconds 1.2e+02) (.yaw _returnvalue))) false false))

(fn ConstructionScript)