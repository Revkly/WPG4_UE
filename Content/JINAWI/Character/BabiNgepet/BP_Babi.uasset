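; BP_Babi is the Babi Ngepet enemy, an AI-driven character that charges forward and damages what it hits.
; Detection overlap with BP_Sakti sets the Blackboard target and updates the AI controller's target distance.
; Charge boosts movement speed and enables AttackHitbox, while Tick drives it forward; hits deal damage and knockback through BPI_Damageable.
; HitDamage always removes one health, syncs the widget bar, then destroys it or briefly blocks AI actions as a stun.
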(event OnComponentBeginOverlap(AttackHitbox)
  (params (OverlappedComponent :type Primitive%20Component%20Object%20Reference) (OtherActor :type Actor%20Object%20Reference) (OtherComp :type Primitive%20Component%20Object%20Reference) (OtherBodyIndex :type Integer) (bFromSweep :type Boolean) (SweepResult :type Hit%20Result%20Structure%20%28by%20ref%29))
  (bind _asbpi_damageable (Utilities|Casting|CastToBPI_Damageable OtherActor))
  (if (not (== OtherActor self))
    (bind _hit_successful (Default|HitDamage _asbpi_damageable 1))
    (if _hit_successful
      (Default|Knockback _asbpi_damageable (Transformation|GetWorldLocation (Variables|Default|GetAttack%20Hitbox)) 1.0))))

(event OnComponentBeginOverlap(Detection)
  (params (OverlappedComponent :type Primitive%20Component%20Object%20Reference) (OtherActor :type Actor%20Object%20Reference) (OtherComp :type Primitive%20Component%20Object%20Reference) (OtherBodyIndex :type Integer) (bFromSweep :type Boolean) (SweepResult :type Hit%20Result%20Structure%20%28by%20ref%29))
  (bind _self self)
  (bind _returnvalue (AI|GetAIController _self))
  (bind _blackboard (Variables|/Script/AIModule.AIController|GetBlackboard _returnvalue))
  (bind _asbp_sakti (Utilities|Casting|CastToBP_Sakti OtherActor))
  (AI|Components|Blackboard|SetValueasObject _blackboard (Utilities|Name|MakeLiteralName "Target") _asbp_sakti)
  (AI|Components|Blackboard|SetValueasBool _blackboard (Utilities|Name|MakeLiteralName "IsPlayerDetected") true)
  (bind _asbp_babi_ngepet_ai (Utilities|Casting|CastToBP_BabiNgepetAI (AI|GetAIController self)))
  (Default|UpdateTargetDistance _asbp_babi_ngepet_ai))

(event Custom|Charge
  (params (Is%20Charging :type Boolean))
  (bind _attack_hitbox (Variables|Default|GetAttack%20Hitbox))
  (bind _charactermovement (Variables|Character|GetCharacterMovement))
  (bind _charactermovement_2 (Variables|Character|GetCharacterMovement))
  (bind _attack_hitbox_2 (Variables|Default|GetAttack%20Hitbox))
  (if Is%20Charging
    (Variables|/Script/Engine.CharacterMovementComponent|SetMaxWalkSpeed _charactermovement_2 3e+03)
    (Variables|/Script/Engine.CharacterMovementComponent|SetMaxAcceleration _charactermovement_2 1e+04)
    (Variables|Default|SetIs%20Charging true)
    (Collision|SetCollisionEnabled _attack_hitbox "QueryOnly")
    (Development|SetHiddeninGame _attack_hitbox false false)
    (else
      (Variables|/Script/Engine.CharacterMovementComponent|SetMaxWalkSpeed _charactermovement 6e+02)
      (Variables|/Script/Engine.CharacterMovementComponent|SetMaxAcceleration _charactermovement 2048.0)
      (Variables|Default|SetIs%20Charging false)
      (Collision|SetCollisionEnabled _attack_hitbox_2 "NoCollision")
      (Development|SetHiddeninGame _attack_hitbox_2 true false))))

(event Custom|Stun
  (bind _returnvalue (Utilities|Name|MakeLiteralName "IsActionBlocked"))
  (bind _self self)
  (bind _returnvalue_2 (AI|GetAIController _self))
  (bind _blackboard (Variables|/Script/AIModule.AIController|GetBlackboard _returnvalue_2))
  (AI|Components|Blackboard|SetValueasBool _blackboard _returnvalue true)
  (Utilities|FlowControl|RetriggerableDelay 0.8)
  (AI|Components|Blackboard|SetValueasBool _blackboard _returnvalue false))

(event EventBeginPlay
  (bind _aswb_health_bar (Utilities|Casting|CastToWB_HealthBar (UserInterface|GetWidget (Variables|Default|GetWidget))))
  (Default|SyncHealthBar _aswb_health_bar (Variables|Default|GetHealth) 9))

(event EventKnockback
  (params (Origin :type Vector :default "0, 0, 0") (Force :type Float%20%28double-precision%29))
  ;[0 0 0 0.171] Knockback
  (Physics|AddImpulse (Variables|Character|GetCharacterMovement) (* (Math|Vector|GetForwardVector (Math|Rotator|FindLookatRotation Origin (Transformation|GetActorLocation))) (* Force "100000.000000,100000.000000,100000.000000")) false))

(event EventTick
  (params (DeltaSeconds :type Float%20%28single-precision%29))
  (if (Variables|Default|GetIs%20Charging)
    (Pawn|Input|AddMovementInput (Math|Vector|GetForwardVector (Math|Rotator|MakeRotator 0.0 0.0 (.yaw (Transformation|GetActorRotation)))) 1.0 false)))

(fn ConstructionScript)

(fn HitDamage
  (params (Damage :type Integer))
  (Audio|PlaySound2D (.OutItem (Utilities|Array|Random (Variables|Default|GetHurt%20Sound))) 1.0 1.0 0.0 0 0)
  (Audio|PlaySound2D "/Game/JINAWI/Sound/Enemy_Hit_General.Enemy_Hit_General" 1.0 1.0 0.0 0 0)
  (Variables|Default|SetHealth (- (Variables|Default|GetHealth) 1))
  (bind _aswb_health_bar (Utilities|Casting|CastToWB_HealthBar (UserInterface|GetWidget (Variables|Default|GetWidget))))
  (Default|SyncHealthBar _aswb_health_bar (Variables|Default|GetHealth) 9)
  (if (<= (Variables|Default|GetHealth) 0)
    (Audio|PlaySound2D (.OutItem (Utilities|Array|Random (Variables|Default|GetDeath%20Sound))) 1.0 1.0 0.0 0 0)
    (Actor|DestroyActor)
    (return true true)
    (else
      (CallFunction|Stun)
      (return true false))))