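; BP_BabiNgepetAI is the AI controller for the Babi Ngepet character, starting the BT_BabiNgepet behavior tree on possession.
; Its UpdateTargetDistance event reads the Target and SelfActor blackboard entries and writes the distance between them to TargetDistance.
; The event stops if either actor is missing and prints the distance as debug output; nothing in this Blueprint calls it.
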(event Custom|Update%20Target%20Distance
  (bind _blackboard (Variables|Default|GetBlackboard))
  (bind _asactor (Utilities|Casting|CastToActor (AI|Components|Blackboard|GetValueasObject _blackboard (Utilities|Name|MakeLiteralName "Target"))))
  (bind _asactor_2 (Utilities|Casting|CastToActor (AI|Components|Blackboard|GetValueasObject _blackboard (Utilities|Name|MakeLiteralName "SelfActor"))))
  (AI|Components|Blackboard|SetValueasFloat (Variables|Default|GetBlackboard) (Utilities|Name|MakeLiteralName "TargetDistance") (Math|Vector|Distance(Vector) (Transformation|GetActorLocation _asactor_2) (Transformation|GetActorLocation _asactor)))
  (Development|PrintString (Utilities|String|ToString(Float) (Math|Vector|Distance(Vector) (Transformation|GetActorLocation _asactor_2) (Transformation|GetActorLocation _asactor)))))

(event EventPossess
  (params (PossessedPawn :type Pawn%20Object%20Reference))
  (AI|RunBehaviorTree "/Game/JINAWI/Character/BabiNgepet/BT_BabiNgepet.BT_BabiNgepet"))

(fn ConstructionScript)